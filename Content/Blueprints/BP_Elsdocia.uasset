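; BP_Elsdocia is a held item, apparently a can, that the custom third-person character can pick up and drop.
; Overlapping its trigger calls TryToPickUp on the character, while Pickup attaches the mesh to the hand socket and disables collision.
; Drop detaches it, enables physics and collision, and restores the saved world location so it does not jump to world origin.
; PrimaryAction only prints a placeholder string.
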(event `self.ReceiveBeginPlay`)

(event `self.ReceiveActorBeginOverlap`
  (params (OtherActor :type "Actor Object Reference")))

(event `self.PickUpTrigger.OnComponentBeginOverlap`
  (params (OverlappedComponent :type "PrimitiveComponent Object Reference") (OtherActor :type "Actor Object Reference") (OtherComp :type "PrimitiveComponent Object Reference") (OtherBodyIndex :type Integer) (bFromSweep :type Boolean) (SweepResult :type "HitResult Structure (by ref)"))
  (bind _asbp_third_person_character_custom (cast `/Game/Blueprints/BP_ThirdPersonCharacterCustom` OtherActor))
  (`/Game/Blueprints/BP_ThirdPersonCharacterCustom.TryToPickUp` _asbp_third_person_character_custom self))

(event `/Game/Blueprints/BPI_Item.Pickup`
  (params (ParentMesh :type "SkeletalMeshComponent Object Reference"))
  (`SceneComponent.K2_AttachToComponent` (`self.elsdocia_game`) ParentMesh "hand_r" "SnapToTarget" "KeepRelative" "KeepRelative" true)
  (`PrimitiveComponent.SetCollisionEnabled` (`self.elsdocia_game`) "NoCollision"))

(event `/Game/Blueprints/BPI_Item.Drop`
  (bind _elsdocia_game (`self.elsdocia_game`))
  (set `self.Drop Location` (`SceneComponent.K2_GetComponentLocation` _elsdocia_game))
  (`SceneComponent.K2_DetachFromComponent` _elsdocia_game "KeepRelative" "KeepRelative" "KeepRelative" true) ; Don't follow the hand anymore
  (`PrimitiveComponent.SetSimulatePhysics` (`self.elsdocia_game`) true) ; use gravity to fall
  (`PrimitiveComponent.SetCollisionEnabled` (`self.elsdocia_game`) "QueryAndPhysics") ; Collide with the ground please
  (`SceneComponent.K2_SetWorldLocation` (`self.elsdocia_game`) (`self.Drop Location`) false false) ; To prevent the can from going to world origin
)

(event `/Game/Blueprints/BPI_Item.PrimaryAction`
  (params (ref_thirdPersonCharCustom :type "/Game/Blueprints/BP_ThirdPersonCharacterCustom Object Reference"))
  (`KismetSystemLibrary.PrintString` "primary"))

(fn `UserConstructionScript`)
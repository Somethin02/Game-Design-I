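; BP_Rat is an enemy rat that chases the player, deals contact damage and dies when stomped.
; PawnSensing triggers an AI MoveTo toward the player character while the rat is alive.
; HitBox overlap damages the custom third-person character and starts its invincibility frames, unless already invincible.
; Sphere overlap while that character is falling shifts the HitBox, flattens the mesh, disables its collision and destroys the rat after a delay.
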(event `self.ReceiveBeginPlay`)

(event `self.Sphere.OnComponentBeginOverlap`
  (params (OverlappedComponent :type "PrimitiveComponent Object Reference") (OtherActor :type "Actor Object Reference") (OtherComp :type "PrimitiveComponent Object Reference") (OtherBodyIndex :type Integer) (bFromSweep :type Boolean) (SweepResult :type "HitResult Structure (by ref)"))
  (bind (_returnvalue_x _returnvalue_y _returnvalue_z) (`KismetMathLibrary.BreakVector` (`SceneComponent.K2_GetComponentLocation` (`self.HitBox`))))
  (bind (_returnvalue_x_2 _returnvalue_y_2 _returnvalue_z_2) (`KismetMathLibrary.BreakVector` (`SceneComponent.K2_GetComponentScale` (`self.street_rat_2k`))))
  (bind _asbp_third_person_character_custom (cast `/Game/Blueprints/BP_ThirdPersonCharacterCustom` OtherActor))
  (if (`NavMovementComponent.IsFalling` (`Character.CharacterMovement` _asbp_third_person_character_custom))
    (`SceneComponent.K2_SetRelativeLocation` (`self.HitBox`) (`KismetMathLibrary.MakeVector` _returnvalue_x (- _returnvalue_y 100.0) _returnvalue_z) false false)
    (set `self.IsDead` true)
    (`SceneComponent.SetRelativeScale3D` (`self.street_rat_2k`) (`KismetMathLibrary.MakeVector` _returnvalue_x_2 _returnvalue_y_2 (/ _returnvalue_z_2 5.0)))
    (`PrimitiveComponent.SetCollisionEnabled` (`self.street_rat_2k`) "NoCollision")
    (`KismetSystemLibrary.Delay` 2.0)
    (`self.K2_DestroyActor`)))

(event `self.PawnSensing.OnSeePawn`
  (params (Pawn :type "Pawn Object Reference"))
  (if (not (`self.IsDead`))
    (`self.FollowPawn`)))

(event `FollowPawn`
  (if (not (`self.IsDead`))
    (`|AIMoveTo` self (0.0 0.0 0.0) (`GameplayStatics.GetPlayerCharacter` 0))))

(event `self.HitBox.OnComponentBeginOverlap`
  (params (OverlappedComponent :type "PrimitiveComponent Object Reference") (OtherActor :type "Actor Object Reference") (OtherComp :type "PrimitiveComponent Object Reference") (OtherBodyIndex :type Integer) (bFromSweep :type Boolean) (SweepResult :type "HitResult Structure (by ref)"))
  (bind _asbp_third_person_character_custom (cast `/Game/Blueprints/BP_ThirdPersonCharacterCustom` OtherActor))
  (if (not (`/Game/Blueprints/BP_ThirdPersonCharacterCustom.Invincibility` _asbp_third_person_character_custom))
    (`GameplayStatics.ApplyDamage` _asbp_third_person_character_custom 10.0)
    (`/Game/Blueprints/BP_ThirdPersonCharacterCustom.InvincibilityFrames` _asbp_third_person_character_custom)))

(fn `UserConstructionScript`)
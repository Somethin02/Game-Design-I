(event `self.ReceiveBeginPlay`
  (`KismetSystemLibrary.PrintString` "Enemy Spawn Manager is Ready")
  (bind _outactors (`GameplayStatics.GetAllActorsOfClass` "/Game/Blueprints/Enemies/BP_GuardSpawner.BP_GuardSpawner_C"))
  (set `self.Spawners` _outactors)
  (`self.Spawn Guards`))

(event `Spawn Guards`
  (for _array_element (`self.Spawners`)
    (bind (_returnvalue_location _returnvalue_rotation) (`KismetMathLibrary.BreakTransform` (`SceneComponent.K2_GetComponentToWorld` (`Actor.RootComponent` _array_element))))
    (bind _returnvalue (`|SpawnActorFromClass` "/Game/Blueprints/Enemies/BP_Guard.BP_Guard_C" (`KismetMathLibrary.MakeTransform` _returnvalue_location _returnvalue_rotation) "Undefined" "MultiplyWithRoot" null null)) ; Create a new enemy at the spawner's location and rotation.
    (set `/Game/Blueprints/Enemies/BP_Guard.Manager` self _returnvalue)
    (`/Engine/EditorBlueprintResources/StandardMacros.IncrementInt` (`self.CurrentEnemyTotal`))))

(event `RemoveGuardAndCheck`
  (`/Engine/EditorBlueprintResources/StandardMacros.DecrementInt` (`self.CurrentEnemyTotal`)
    (:`  `
      (if (not (> (`self.CurrentEnemyTotal`) 0))
        (`KismetSystemLibrary.PrintString` "You may pass!" true true (struct :`G` 0.66 :`B` 1.0 :`A` 1.0) 5.0)))))

(fn `UserConstructionScript`)
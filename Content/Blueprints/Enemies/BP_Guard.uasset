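; BP_Guard is an enemy guard that only a player armed with the sword can defeat.
; When the custom third-person character overlaps its capsule while armed, the body switches to physics simulation and, after a short delay, the guard notifies its manager and destroys itself.
; An unarmed player only gets a printed warning that the legendary Sword is required to pass.
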(event `self.Capsule.OnComponentBeginOverlap`
  (params (OverlappedComponent :type "PrimitiveComponent Object Reference") (OtherActor :type "Actor Object Reference") (OtherComp :type "PrimitiveComponent Object Reference") (OtherBodyIndex :type Integer) (bFromSweep :type Boolean) (SweepResult :type "HitResult Structure (by ref)"))
  (bind _asbp_third_person_character_custom (cast `/Game/Blueprints/BP_ThirdPersonCharacterCustom` OtherActor))
  (if (`/Game/Blueprints/BP_ThirdPersonCharacterCustom.IsArmed` _asbp_third_person_character_custom)
    (`KismetSystemLibrary.PrintString` "Ouch")
    (`PrimitiveComponent.SetSimulatePhysics` (`self.Body`) true)
    (`KismetSystemLibrary.Delay` 2.0)
    (`/Game/Blueprints/Enemies/BP_GuardSpawnManager.RemoveGuardAndCheck` (`self.Manager`))
    (`self.K2_DestroyActor`)
    (else
      (`KismetSystemLibrary.PrintString` "Only one with the legendary Sword can pass!"))))

(fn `UserConstructionScript`)
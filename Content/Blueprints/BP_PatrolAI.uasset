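; Enemy AI that wanders between tagged patrol points and chases the player once it sees a pawn.
; A timed self-calling event moves it to one of four randomly indexed PatrolPoint actors until PawnSensing flags pursuit and sends it toward the player.
; Hitbox overlap damages the custom third-person character and starts its invincibility frames, unless already invincible.
; Deactivation of PawnSensing clears pursuit, greatly widens its sight settings and resumes patrolling.
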(event `self.ReceiveBeginPlay`
  (bind _outactors (`GameplayStatics.GetAllActorsOfClassWithTag` "/Script/Engine.Actor" "PatrolPoint"))
  (`self.MoveToPatrolPoint`))

(event `MoveToPatrolPoint`
  (if (not (`self.InPursuit?`))
    (`|AIMoveTo` self (`self.K2_GetActorLocation` (`|GetArrayItem` (stale `self.ReceiveBeginPlay` _outactors) (`self.CurrentPatrolPoint`))) null 200.0
      (:`then`
        _)
      (:`OnSuccess`
        _)
      (:`OnFail`
        _))
    (`KismetSystemLibrary.Delay` 7.0)
    (set `self.CurrentPatrolPoint` (`KismetMathLibrary.RandomInteger` 4))
    (`self.MoveToPatrolPoint`)))

(event `MoveToPlayer`
  (`|AIMoveTo` self (0.0 0.0 0.0) (`GameplayStatics.GetPlayerCharacter` 0) 0.0
    (:`then`
      _)
    (:`OnSuccess`
      _)
    (:`OnFail`
      _))
  (`KismetSystemLibrary.Delay` 0.2))

(event `self.Hitbox.OnComponentBeginOverlap`
  (params (OverlappedComponent :type "PrimitiveComponent Object Reference") (OtherActor :type "Actor Object Reference") (OtherComp :type "PrimitiveComponent Object Reference") (OtherBodyIndex :type Integer) (bFromSweep :type Boolean) (SweepResult :type "HitResult Structure (by ref)"))
  (bind _asbp_third_person_character_custom (cast `/Game/Blueprints/BP_ThirdPersonCharacterCustom` OtherActor))
  (if (not (`/Game/Blueprints/BP_ThirdPersonCharacterCustom.Invincibility` _asbp_third_person_character_custom))
    (`GameplayStatics.ApplyDamage` _asbp_third_person_character_custom 100.0)
    (`/Game/Blueprints/BP_ThirdPersonCharacterCustom.InvincibilityFrames` _asbp_third_person_character_custom)))

(event `self.PawnSensing.OnSeePawn`
  (params (Pawn :type "Pawn Object Reference"))
  (set `self.InPursuit?` true)
  (`self.MoveToPlayer`))

(event `self.PawnSensing.OnComponentDeactivated`
  (params (Component :type "ActorComponent Object Reference"))
  (set `self.InPursuit?` false)
  (set `PawnSensingComponent.SightRadius` 1000000000.0 (`self.PawnSensing`))
  (`PawnSensingComponent.SetPeripheralVisionAngle` (`self.PawnSensing`) 360.0)
  (`PawnSensingComponent.SetPeripheralVisionAngle` (`self.PawnSensing`) 360.0)
  (`self.MoveToPatrolPoint`))

(fn `UserConstructionScript`)